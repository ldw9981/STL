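; BP_Enemy is an enemy Blueprint that tracks health and shows it on an HP bar widget.
; It starts at max health, subtracts incoming damage and sends the health ratio to UMG_HPBar.
; At zero health or below, it calls a state-change event with the second monster-state enum value.
; That event stores the state and checks the controller's validity, with nothing wired after the check.
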(event Custom|상태변경
  (params (몬스터상태 :type 몬스터상태열거형%20Enum :default "NewEnumerator0"))
  (Variables|Default|Set현재상태_BP 몬스터상태)
  (Utilities|IsValid (Pawn|GetController)))

(event EventBeginPlay
  (Variables|Default|Set현재체력 (Variables|Default|Get최대체력)))

(event Collision|EventActorBeginOverlap
  (params (OtherActor :type Actor%20Object%20Reference)))

(event EventTick
  (params (DeltaSeconds :type Float%20%28single-precision%29)))

(event Game|Damage|EventAnyDamage
  (params (Damage :type Float%20%28single-precision%29) (DamageType :type Damage%20Type%20Object%20Reference) (InstigatedBy :type Controller%20Object%20Reference) (DamageCauser :type Actor%20Object%20Reference))
  (Variables|Default|Set현재체력 (- (Variables|Default|Get현재체력) Damage))
  (bind _asumg_hpbar (Utilities|Casting|CastToUMG_HPBar (UserInterface|GetUserWidgetObject (Variables|Default|GetHPBar))))
  (Default|체력바게이지전달 _asumg_hpbar (/ (Variables|Default|Get현재체력) (Variables|Default|Get최대체력)))
  (if (not (> (Variables|Default|Get현재체력) 0.0))
    (CallFunction|상태변경 "NewEnumerator1")))

(fn ConstructionScript)