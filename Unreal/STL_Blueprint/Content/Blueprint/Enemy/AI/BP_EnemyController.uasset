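; BP_EnemyController is the AI controller that starts enemy behavior when it possesses a pawn.
; On possess, it initializes the BP_EnemyBB blackboard and seeds it with a wait duration and the pawn's current location.
; It then runs the BP_EnemyBT behavior tree, with no other active logic in the controller itself.
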(event EventBeginPlay)

(event EventTick
  (params (DeltaSeconds :type Float%20%28single-precision%29)))

(event EventOnPossess
  (params (PossessedPawn :type Pawn%20Object%20Reference))
  (Utilities|FlowControl|Sequence
    (:then_0
      (Class|AIController|UseBlackboard "/Game/Blueprint/Enemy/AI/BP_EnemyBB.BP_EnemyBB")
      (AI|Components|Blackboard|SetValueasFloat (Variables|Default|GetBlackboard) (Variables|Default|Get대시기간%20이름) 3.0)
      (AI|Components|Blackboard|SetValueasVector (Variables|Default|GetBlackboard) (Variables|Default|Get현재위치%20이름) (Transformation|GetActorLocation (Pawn|GetControlledPawn))))
    (:then_1
      (AI|RunBehaviorTree "/Game/Blueprint/Enemy/AI/BP_EnemyBT.BP_EnemyBT"))))

(fn ConstructionScript)