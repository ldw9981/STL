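; Character Blueprint that handles movement and a four-stage melee combo, switched by a peace/attack state (평화/공격).
; In the peace state, Tick turns the controller toward world-axis input and moves forward along it.
; DoAttack starts the montage or queues the next section name in NextSection, and AttackEnd restores peace.
; Separate events add a forward dash impulse and apply sphere-trace damage; the HP-bar billboarding event is unused backup.
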(event Custom|DoAttack
  (bind _mesh (Variables|Character|GetMesh))
  (bind _returnvalue (Components|SkeletalMesh|GetAnimInstance _mesh))
  ;[1 1 1] 캐릭터 공격
  (Variables|Default|SetState_BP "NewEnumerator1")
  (if (Animation|Montage|MontageIsPlaying _returnvalue "/Game/Characters/Animations/SK_Mannequin_Skeleton_Montage.SK_Mannequin_Skeleton_Montage")
    (switch name (Animation|Montage|MontageGetCurrentSection _returnvalue "/Game/Characters/Animations/SK_Mannequin_Skeleton_Montage.SK_Mannequin_Skeleton_Montage")
      (:Default
        (Variables|Default|SetNextSection "None"))
      (:공격1
        (Variables|Default|SetNextSection "공격2"))
      (:공격2
        (Variables|Default|SetNextSection "공격3"))
      (:공격3
        (Variables|Default|SetNextSection "공격4")))
    (else
      (Animation|Montage|MontagePlay (Components|SkeletalMesh|GetAnimInstance (Variables|Character|GetMesh)) "/Game/Characters/Animations/SK_Mannequin_Skeleton_Montage.SK_Mannequin_Skeleton_Montage" 1.0 "MontageLength" 0.0 true))))

(event Custom|AttackEnd
  ;[1 1 1] 공격 종료
  (Variables|Default|SetState_BP "NewEnumerator0"))

(event Custom|공격대시
  ;[1 1 1] 공격 대시
  (Physics|AddImpulse (Variables|Character|GetCharacterMovement) (* (Transformation|GetActorForwardVector) (Variables|Default|Get대시파워)) true))

(event Custom|빌보딩
  ;[1 1 1] 빌보딩 - 코드 백업
  (Transformation|SetWorldRotation (Variables|Default|GetHPBar) (Math|Rotator|MakeRotfromX (- (Camera|GetCameraLocation (Game|GetPlayerCameraManager 0)) (Transformation|GetActorLocation))) false false))

(event Custom|공격판정
  (bind _returnvalue (Transformation|GetActorLocation))
  (bind (_outhit _returnvalue_2) (Collision|SphereTraceForObjects _returnvalue (+ _returnvalue (* (Transformation|GetActorForwardVector) 1.8e+02)) 6e+01 (Utilities|Array|MakeArray "ObjectTypeQuery3") false 0 "ForDuration"))
  (if _returnvalue_2
    (Game|Damage|ApplyDamage (.HitActor (Collision|BreakHitResult _outhit)) 2e+01 (Pawn|GetController) self)))

(event EventTick
  (params (DeltaSeconds :type Float%20%28single-precision%29))
  ;[1 1 1] 캐릭터 이동
  (switch Utilities|FlowControl|Switch|SwitchonECharacterStates (Variables|Default|GetState_BP)
    (:NewEnumerator0
      (if (or (!= (Input|AxisValues|GetUpDown) 0.0) (!= (Input|AxisValues|GetLeftRight) 0.0))
        (Pawn|SetControlRotation (Pawn|GetController) (Math|Rotator|MakeRotfromX (Math|Vector|MakeVector (Input|AxisValues|GetUpDown) (Input|AxisValues|GetLeftRight) 0.0)))
        (Pawn|Input|AddMovementInput (Transformation|GetActorForwardVector (Pawn|GetController)) 1.0 false)))))

(fn ConstructionScript)