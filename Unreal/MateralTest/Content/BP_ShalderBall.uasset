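; BP_ShalderBall is an actor that animates a dissolve material on its static mesh over time.
; The construction script creates a dynamic instance of M_Dissolve_Inst on element 0, and BeginPlay sets its Noises texture from the Basecolor variable.
; Tick accumulates a tenth of delta time into TotalTime and writes it to the Cut parameter, with no clamp or reset.
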(event EventBeginPlay
  (Rendering|Material|SetTextureParameterValue (Variables|Default|GetMaterialInstance) "Noises" "/Game/Materials/basecolor.basecolor"))

(event Collision|EventActorBeginOverlap
  (params (OtherActor :type Actor%20Object%20Reference)))

(event EventTick
  (params (DeltaSeconds :type Float%20%28single-precision%29))
  (bind _output_get (Variables|Default|SetTotalTime (+ (/ DeltaSeconds 1e+01) (Variables|Default|GetTotalTime))))
  (Rendering|Material|SetScalarParameterValue (Variables|Default|GetMaterialInstance) "Cut" _output_get :!class /Script/Engine.MaterialInstanceDynamic))

(fn ConstructionScript
  (bind _returnvalue (Rendering|Material|CreateDynamicMaterialInstance (Variables|Default|GetStaticMesh) 0 "/Game/Materials/ShaderBall/M_Dissolve_Inst.M_Dissolve_Inst" "None" :!class /Script/Engine.PrimitiveComponent))
  (Variables|Default|SetMaterialInstance _returnvalue))