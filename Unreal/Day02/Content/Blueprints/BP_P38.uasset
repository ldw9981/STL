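; BP_P38 is a player-controlled P-38 plane pawn that flies along its forward vector and fires rockets.
; Each tick it spins the left and right propellers by a delta-time-scaled speed and feeds the Boost axis into movement input.
; Pitch and Roll axes add local actor rotation directly, without delta-time scaling.
; Pressing Fire spawns BP_Rocket at the Arrow component's transform and increments the shot count in BP_GameMode.
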(event Custom|RotatePropeller
  (params (Propeller :type Static%20Mesh%20Component%20Object%20Reference) (Speed :type Float%20%28single-precision%29))
  (Transformation|AddLocalRotation Propeller (Math|Rotator|MakeRotator (* Speed (Utilities|Time|GetWorldDeltaSeconds)) 0.0 0.0) false false))

(event EventBeginPlay)

(event Collision|EventActorBeginOverlap
  (params (OtherActor :type Actor%20Object%20Reference)))

(event EventTick
  (params (DeltaSeconds :type Float%20%28single-precision%29))
  (CallFunction|RotatePropeller (Variables|Default|GetLeft) (Variables|Speed|GetPropellerSpeed))
  (CallFunction|RotatePropeller (Variables|Default|GetRight) (Variables|Speed|GetPropellerSpeed))
  (Pawn|Input|AddMovementInput (Transformation|GetActorForwardVector) (Input|AxisValues|GetBoost) false))

(event Input|ActionEvents|InputActionFire
  (params (Key :type Key%20Structure))
  (:Pressed
    (Game|SpawnActorfromClass "/Game/Blueprints/BP_Rocket.BP_Rocket_C" (Transformation|GetWorldTransform (Variables|Default|GetArrow)) "Undefined" 0 0)
    (bind _asbp_game_mode (Utilities|Casting|CastToBP_GameMode (Game|GetGameMode)))
    (Default|AddShootCount _asbp_game_mode)))

(event Input|AxisEvents|InputAxisBoost
  (params (AxisValue :type Float%20%28single-precision%29)))

(event Input|AxisEvents|InputAxisPitch
  (params (AxisValue :type Float%20%28single-precision%29))
  (Transformation|AddActorLocalRotation (Math|Rotator|MakeRotator 0.0 AxisValue 0.0) false false))

(event Input|AxisEvents|InputAxisRoll
  (params (AxisValue :type Float%20%28single-precision%29))
  (Transformation|AddActorLocalRotation (Math|Rotator|MakeRotator AxisValue 0.0 0.0) false false))

(fn ConstructionScript)