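; P-38 aircraft Blueprint that flies itself forward along local X and spins its two propellers.
; Tick scales PropellerSpeed, set in the construction script, by delta time, rolls Left and Right, then offsets the actor at a constant rate.
; Rotation goes through a custom event, commented as syncable, wrapping RotatePropeller; the direct local-only calls are left disconnected.
; Pressing W applies a fixed roll and pitch step to the plane.
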(event Custom|RotatePropeller2
  (params (Propeller :type Static%20Mesh%20Component%20Object%20Reference) (Speed :type Float%20%28single-precision%29))
  (CallFunction|RotatePropeller Propeller Speed))

(event EventTick
  (params (DeltaSeconds :type Float%20%28single-precision%29))
  (Utilities|FlowControl|Sequence
    (:then_0
      ;[1 1 1] 속도값 계싼
      (Variables|Default|SetResultSpeed (* DeltaSeconds (Variables|Speed|GetPropellerSpeed))))
    (:then_1
      ;[1 1 1] 동기화 가능한 프로펠러 회전
      (CallFunction|RotatePropeller2 (Variables|Default|GetLeft) (Variables|Default|GetResultSpeed))
      (CallFunction|RotatePropeller2 (Variables|Default|GetRight) (Variables|Default|GetResultSpeed)))
    (:then_2
      ;[1 1 1] 비행기 이동
      (Transformation|AddActorLocalOffset (Math|Vector|MakeVector (* (Utilities|Time|GetWorldDeltaSeconds) 3e+01) 0.0 0.0) false false))))

(event Input|KeyboardEvents|W
  (params (Key :type Key%20Structure))
  (:Pressed
    (Transformation|AddActorLocalRotation self (Math|Rotator|MakeRotator 1e+01 1e+01 0.0) false false)))

(event Input|KeyboardEvents|S
  (params (Key :type Key%20Structure)))

(fn ConstructionScript
  (Variables|Speed|SetPropellerSpeed 1.5e+03))

(fn RotatePropeller
  (params (Propeller :type Static%20Mesh%20Component%20Object%20Reference) (Speed :type Float%20%28single-precision%29))
  (Transformation|AddRelativeRotation Propeller (Math|Rotator|MakeRotator Speed 0.0 0.0) false false))

(fn NewFunction0
  (Transformation|AddRelativeRotation (Variables|Default|GetLeft) (Math|Rotator|MakeRotator 1e+01 0.0 0.0) false false))