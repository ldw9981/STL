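; BP_Arrow is an arrow projectile that stops and sticks to the actor it overlaps.
; When its Capsule begins an overlap, a sequence prints the other actor's class name, then zeroes the ProjectileMovement velocity and gravity.
; It then attaches itself to the overlapped actor, keeping its world transform, and disables capsule collision.
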(event OnComponentBeginOverlap(Capsule)
  (params (OverlappedComponent :type Primitive%20Component%20Object%20Reference) (OtherActor :type Actor%20Object%20Reference) (OtherComp :type Primitive%20Component%20Object%20Reference) (OtherBodyIndex :type Integer) (bFromSweep :type Boolean) (SweepResult :type Hit%20Result%20Structure%20%28by%20ref%29))
  (bind _projectilemovement (Variables|Default|GetProjectileMovement))
  (Utilities|FlowControl|Sequence
    (:then_0
      (Development|PrintString (Utilities|GetClassDisplayName (Utilities|GetClass OtherActor))))
    (:then_1
      (Game|Components|ProjectileMovement|SetVelocityinLocalSpace _projectilemovement "0, 0, 0")
      (Variables|/Script/Engine.ProjectileMovementComponent|SetProjectileGravityScale _projectilemovement 0.0))
    (:then_2
      (Transformation|AttachActorToActor (Variables|Default|GetOverlapOtherActor) "None" "KeepWorld" "KeepWorld" "KeepWorld" true)
      (Collision|SetCollisionEnabled (Variables|Default|GetCapsule) "NoCollision"))))

(event EventBeginPlay)

(event Collision|EventActorBeginOverlap
  (params (OtherActor :type Actor%20Object%20Reference)))

(event EventTick
  (params (DeltaSeconds :type Float%20%28single-precision%29)))

(fn ConstructionScript)