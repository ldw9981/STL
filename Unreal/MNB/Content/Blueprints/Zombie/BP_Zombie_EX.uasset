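; BP_Zombie_EX is an AI zombie character that chases living Player-tagged pawns it sees.
; On possession it sets up the BB_Zombie_2 blackboard and runs BT_Zombie_2.
; While Normal, PawnSensing stores the target in the blackboard and switches the custom state component to Chase.
; State changes set walk or run speed and mirror CurrentState to the blackboard, and the billboard HP widget receives the state component at BeginPlay.
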(event OnSeePawn(PawnSensing)
  (params (Pawn :type Pawn%20Object%20Reference))
  (bind _returnvalue (Actor|GetComponentbyClass Pawn "/Script/MNB.CharacterStateComponent"))
  (if (Utilities|Enum|Equal(Enum) (Variables|/Script/MNB.CharacterStateComponent|GetCurrentState (Variables|Default|GetBP_CustomState)) "Normal")
    (if (Actor|ActorHasTag Pawn "Player")
      (if (Utilities|IsValid _returnvalue)
        (if (not (Utilities|Enum|Equal(Enum) (Variables|/Script/MNB.CharacterStateComponent|GetCurrentState _returnvalue) "Dead"))
          (bind _output_get (Variables|Default|SetBlackBoardKey "ChaseTargetActor"))
          (AI|Components|Blackboard|SetValueasObject (Variables|Default|GetBlackBoard) _output_get Pawn)
          (Variables|/Script/MNB.CharacterStateComponent|SetCurrentState (Variables|Default|GetBP_CustomState) "Chase"))))))

(event OnChangeCharacterState(BP_CustomState)
  (params (VariableName :type Name :default "None"))
  (bind _bp_customstate (Variables|Default|GetBP_CustomState))
  (bind _currentstate (Variables|/Script/MNB.CharacterStateComponent|GetCurrentState _bp_customstate))
  (switch string (Utilities|String|ToString(Name) VariableName)
    (:CurrentState
      (Utilities|FlowControl|Sequence
        (:then_0
          (switch Utilities|FlowControl|Switch|SwitchonECharacterState (Variables|/Script/MNB.CharacterStateComponent|GetCurrentState (Variables|Default|GetBP_CustomState))
            (:Normal
              (Variables|/Script/Engine.CharacterMovementComponent|SetMaxWalkSpeed (Variables|Character|GetCharacterMovement) (Variables|Default|GetWalkSpeed)))
            (:Chase
              (Variables|/Script/Engine.CharacterMovementComponent|SetMaxWalkSpeed (Variables|Character|GetCharacterMovement) (Variables|Default|GetRunSpeed)))))
        (:then_1
          (bind _output_get (Variables|Default|SetBlackBoardKey "CurrentState"))
          (AI|Components|Blackboard|SetValueasEnum (Variables|Default|GetBlackBoard) _output_get _currentstate)
          (Development|PrintString (Utilities|String|EnumtoString _currentstate)))))))

(event EventBeginPlay
  (bind _asumg_zombie_hp (Utilities|Casting|CastToUMG_ZombieHP (UserInterface|GetUserWidgetObject (Variables|Default|GetBillboardWidget))))
  (Variables|/Game/Blueprints/Zombie/UI/UMG_ZombieHP.UMG_ZombieHP_C|SetCharacterState _asumg_zombie_hp (Variables|Default|GetBP_CustomState)))

(event Collision|EventActorBeginOverlap
  (params (OtherActor :type Actor%20Object%20Reference)))

(event EventTick
  (params (DeltaSeconds :type Float%20%28single-precision%29)))

(event EventPossessed
  (params (NewController :type Controller%20Object%20Reference))
  (bind _asaicontroller (Utilities|Casting|CastToAIController NewController))
  (Utilities|FlowControl|Sequence
    (:then_0
      (bind _blackboardcomponent (Class|AIController|UseBlackboard _asaicontroller "/Game/Blueprints/Zombie/AI/BB_Zombie_2.BB_Zombie_2"))
      (Variables|Default|SetBlackBoard _blackboardcomponent))
    (:then_1
      (AI|RunBehaviorTree _asaicontroller "/Game/Blueprints/Zombie/AI/BT_Zombie_2.BT_Zombie_2"))))

(fn ConstructionScript)