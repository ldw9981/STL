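; BP_Actor_Arrow is an arrow projectile that stops and sticks to whatever actor its capsule overlaps.
; On overlap, it stores the other actor, zeroes velocity and gravity, then attaches to that actor keeping its world transform.
; Capsule collision is disabled only when the target is a Character, which a note links to whether the arrow is retrievable.
; A blocking hit only zeroes velocity and speed limits and prints a debug message.
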(event OnComponentHit(Capsule)
  (params (HitComponent :type Primitive%20Component%20Object%20Reference) (OtherActor :type Actor%20Object%20Reference) (OtherComp :type Primitive%20Component%20Object%20Reference) (NormalImpulse :type Vector :default "0, 0, 0") (Hit :type Hit%20Result%20Structure%20%28by%20ref%29))
  (bind _projectilemovement (Variables|Default|GetProjectileMovement))
  (Game|Components|ProjectileMovement|SetVelocityinLocalSpace _projectilemovement "0, 0, 0")
  (Variables|/Script/Engine.ProjectileMovementComponent|SetInitialSpeed _projectilemovement 0.0)
  (Variables|/Script/Engine.ProjectileMovementComponent|SetMaxSpeed _projectilemovement 0.0)
  (Development|PrintString "hit"))

(event OnComponentBeginOverlap(Capsule)
  (params (OverlappedComponent :type Primitive%20Component%20Object%20Reference) (OtherActor :type Actor%20Object%20Reference) (OtherComp :type Primitive%20Component%20Object%20Reference) (OtherBodyIndex :type Integer) (bFromSweep :type Boolean) (SweepResult :type Hit%20Result%20Structure%20%28by%20ref%29))
  (bind _projectilemovement (Variables|Default|GetProjectileMovement))
  (Utilities|FlowControl|Sequence
    (:then_0
      (Variables|Default|SetOverlapOtherActor OtherActor))
    (:then_1
      ;[1 1 1] 반드시 있어야 정지
      (Game|Components|ProjectileMovement|SetVelocityinLocalSpace _projectilemovement "0, 0, 0")
      (Variables|/Script/Engine.ProjectileMovementComponent|SetProjectileGravityScale _projectilemovement 0.0)
      (Transformation|AttachActorToActor (Variables|Default|GetOverlapOtherActor) "None" "KeepWorld" "KeepWorld" "KeepWorld" true)
      ;[1 1 1] 회수불가 or 회수가능
      (Utilities|Casting|CastToCharacter (Variables|Default|GetOverlapOtherActor))
      (Collision|SetCollisionEnabled (Variables|Default|GetCapsule) "NoCollision"))))

(event EventBeginPlay)

(event Collision|EventActorBeginOverlap
  (params (OtherActor :type Actor%20Object%20Reference)))

(event EventTick
  (params (DeltaSeconds :type Float%20%28single-precision%29)))

(fn ConstructionScript)